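; Formation actor that spawns a group of units in ranked lines and moves them together between positions.
; Two points set centre, facing and width; generated grid slots are rotated, stored per unit and sent as slightly randomized navigable destinations.
; MoveFormation issues an intermediate move, busy-loops while units move, then issues the final one.
; Tick tracks movement, turns slower units toward the target point and feeds a test offset to Niagara.
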(event EventBeginPlay)

(event Collision|EventActorBeginOverlap
  (params (OtherActor :type Actor%20Object%20Reference)))

(event EventTick
  (params (DeltaSeconds :type Float%20%28single-precision%29))
  (CallFunction|CheckFormationMovement)
  (Niagara|SetNiagaraVariable(Vector3) (Variables|Default|GetNiagaraSystem) "PositionOffset" (Variables|Default|GetniagaraTestOffset))
  (Variables|Default|SetniagaraTestOffset (+ (Variables|Default|GetniagaraTestOffset) (Class|KismetMathLibrary|VectorOne))))

(event EventParticleData
  (params (Data :type Array%20of%20Basic%20Particle%20Data%20Structures) (NiagaraSystem :type Niagara%20System%20Object%20Reference))
  (Development|PrintString (Utilities|String|ToString(Integer) (Utilities|Array|Length Data))))

(fn ConstructionScript
  (for _array_element 0
    (LocalVariables|Setcentre (+ (Transformation|GetWorldLocation (Variables|/Script/Engine.Character|GetCapsuleComponent _array_element)) (LocalVariables|Getcentre)))))

(fn GenerateLineFormation
  (params (unitCount :type Integer) (Width :type Integer))
  (bind _spread (Variables|Default|Getspread))
  (for _index (range 0 (- unitCount 1))
    (if (== (Math|Integer|%(Integer) _index Width) 0)
      (Math|Float|DecrementFloat (LocalVariables|GetverticalOffset)
        (:%20%20
          (LocalVariables|SethorizontalOffset (+ (/ (Math|Conversions|ToFloat(Integer) Width) -2.0) 0.5))))
      (else
        (Math|Float|IncrementFloat (LocalVariables|GethorizontalOffset)
          (:%20%20
            _))))
    (Utilities|Array|Add (LocalVariables|GetformationCords) (Math|Vector|MakeVector (* (LocalVariables|GetverticalOffset) _spread) (* (LocalVariables|GethorizontalOffset) _spread) 5.0)))
  (return (LocalVariables|GetformationCords)))

(fn AngleBetweenVectors
  (params (vector1 :type Vector) (vector2 :type Vector))
  (bind _returnvalue (Math|Vector|Normalize vector2))
  (bind _returnvalue_2 (Math|Vector|Normalize vector1))
  (bind _returnvalue_3 (Math|Vector|DotProduct _returnvalue_2 _returnvalue))
  (bind _returnvalue_4 (Class|KismetMathLibrary|DegAcos _returnvalue_3))
  (Development|PrintString (Utilities|String|ToString(Float) _returnvalue_4))
  (return _returnvalue_4))

(fn RotationArrow
  (params (X :type Float%20%28single-precision%29) (Y :type Float%20%28single-precision%29) (range :type Float%20%28single-precision%29) (angle :type Rotator))
  (return (+ X (* range (Math|Trig|Cos(Degrees) (.yaw angle)))) (+ Y (* range (Math|Trig|Sin(Degrees) (.yaw angle))))))

(fn PointwithRotation
  (params (angle :type Float%20%28single-precision%29) (centerPoint :type Vector) (targetPoint :type Vector))
  (bind _returnvalue (Math|Trig|Cos(Degrees) angle))
  (bind _returnvalue_2 (Math|Trig|Sin(Degrees) angle))
  (bind _returnvalue_3 (- (.y targetPoint) (.y centerPoint)))
  (bind _returnvalue_4 (- (.x targetPoint) (.x centerPoint)))
  (return (Math|Vector|MakeVector (+ (- (* _returnvalue _returnvalue_4) (* _returnvalue_2 _returnvalue_3)) (.x centerPoint)) (+ (* _returnvalue_4 _returnvalue_2) (* _returnvalue_3 _returnvalue) (.y centerPoint)) (.z targetPoint))))

(fn SpawnFormation
  (params (unitCount :type Integer) (Width :type Integer) (formationStartingPoint :type Vector) (owner :type Vive%20Pawn%20Character%20Object%20Reference))
  (bind _formation (Variables|Default|Getformation))
  (bind _formation_2 (Variables|Default|Getformation))
  (bind _returnvalue (Niagara|SpawnSystematLocation "/Game/Blueprints/Niagara/FormationSystem.FormationSystem" formationStartingPoint))
  (Variables|Default|SetNiagaraSystem _returnvalue)
  (Class|NiagaraComponent|SetVariableObject _returnvalue "ReferenceBlueprint" self)
  (Variables|Default|SetunitNumber unitCount)
  (bind _formationpositions (CallFunction|GenerateLineFormation unitCount Width))
  (for _array_element _formationpositions
    (bind _returnvalue_2 (Game|SpawnActorfromClass "/Game/Blueprints/Unit/Unit.Unit_C" (Math|Transform|MakeTransform (+ formationStartingPoint _array_element) "0, 0, 0" "1,1,1") "AlwaysSpawn" owner owner 0))
    (Utilities|Array|Add _formation (Utilities|Struct|MakeUnitFormationParam _array_element _returnvalue_2 "0.000000,0.000000,0.000000" (Transformation|GetActorLocation _returnvalue_2)))
    (Variables|Default|SetformationCenter (+ (Transformation|GetActorLocation _returnvalue_2) (Variables|Default|GetformationCenter))))
  (Variables|Default|SetformationCenter (/ (Variables|Default|GetformationCenter) (Utilities|Array|Length _formation)))
  (for _array_element_2 _formation_2
    (for _array_element_3 _formation_2
      (Collision|IgnoreActorwhenMoving (Variables|/Script/Engine.Character|GetCapsuleComponent (.unit _array_element_2)) (.unit _array_element_3) true))
    (Variables|/Script/Engine.CharacterMovementComponent|SetMaxWalkSpeed (Variables|/Script/Engine.Character|GetCharacterMovement (.unit _array_element_2)) 2e+02)))

(fn PositionFormation
  (params (target :type Vector) (rotation :type Rotator))
  (bind _formation (Variables|Default|Getformation))
  (Variables|Default|SetnewFormationRotation rotation)
  (Variables|Default|SetnewFormationCenter target)
  (for (_array_element _array_index) _formation
    (bind _point_ (CallFunction|PointwithRotation (.Yaw (Math|Rotator|BreakRotator (Variables|Default|GetnewFormationRotation))) (Variables|Default|GetnewFormationCenter) (+ (.unitvector _array_element) (Variables|Default|GetnewFormationCenter))))
    (Utilities|Array|SetArrayElem _formation _array_index (Utilities|Struct|MakeUnitFormationParam (.unitvector _array_element) (.unit _array_element) (Variables|Default|GetnewFormationRotation) _point_ 0 0))))

(fn MoveFormation
  (params (pos1 :type Vector) (pos2 :type Vector) (targetPoint :type Vector))
  (bind _formation (Variables|Default|Getformation))
  (bind _formation_2 (Variables|Default|Getformation))
  (bind (_pos1_ _pos2_) (CallFunction|CalculateFirstFormationPosition pos1 pos2))
  (CallFunction|DynamicPositionFormation _pos1_ _pos2_)
  (for (_array_element _array_index) _formation_2
    (bind _asunit (Utilities|Casting|CastToUnit (.unit _array_element)))
    (Default|MoveUnit _asunit (Math|Vector2D|MakeVector2D (.x (.RandomLocation (Class|NavigationSystemV1|GetRandomPointinNavigableRadius (.unittemplocation _array_element) 5.0 0 0))) (.y (.RandomLocation (Class|NavigationSystemV1|GetRandomPointinNavigableRadius (.unittemplocation _array_element) 5.0 0 0)))))
    (Utilities|Array|SetArrayElem _formation_2 _array_index (Utilities|Struct|MakeUnitFormationParam (.unitvector _array_element) (.unit _array_element) (Variables|Default|GetnewFormationRotation) (.unittemplocation _array_element) 0 0)))
  (Variables|Default|SetformationCenter (Variables|Default|GetnewFormationCenter))
  (Variables|Default|SetformationRotation (Variables|Default|GetnewFormationRotation))
  (while (Variables|Default|GetformationMoving)
    (Development|PrintString "STILL MOVING"))
  (CallFunction|DynamicPositionFormation pos1 pos2)
  (for (_array_element_2 _array_index_2) _formation
    (bind _asunit_2 (Utilities|Casting|CastToUnit (.unit _array_element_2)))
    (Default|MoveUnit _asunit_2 (Math|Vector2D|MakeVector2D (.x (.RandomLocation (Class|NavigationSystemV1|GetRandomPointinNavigableRadius (.unittemplocation _array_element_2) 5.0 0 0))) (.y (.RandomLocation (Class|NavigationSystemV1|GetRandomPointinNavigableRadius (.unittemplocation _array_element_2) 5.0 0 0)))))
    (Utilities|Array|SetArrayElem _formation _array_index_2 (Utilities|Struct|MakeUnitFormationParam (.unitvector _array_element_2) (.unit _array_element_2) (Variables|Default|GetnewFormationRotation) (.unittemplocation _array_element_2) 0 0))))

(fn DynamicPositionFormation
  (params (startPoint :type Vector) (endPoint :type Vector))
  (bind _formation (Variables|Default|GetFormation))
  (bind _temppositions (LocalVariables|GettempPositions))
  (bind _rotatedpos (LocalVariables|GetrotatedPos))
  (LocalVariables|SetstartPos startPoint)
  (LocalVariables|SetendPos endPoint)
  (LocalVariables|SetdistanceStartEnd (Math|Vector|Distance(Vector) startPoint endPoint))
  (Variables|Default|SetnewFormationCenter (/ (+ startPoint endPoint) 2.0))
  (Variables|Default|SetformationRotation (Math|Rotator|MakeRotator 0.0 0.0 (- (.yaw (Math|Rotator|FindLookatRotation (LocalVariables|GetstartPos) (LocalVariables|GetendPos))) 9e+01)))
  (bind _spacing (CallFunction|CalculateSpacing))
  (bind _output_get (Variables|Default|Setspacing _spacing))
  (if (> (LocalVariables|GetdistanceStartEnd) (Variables|Default|Getspacing))
    (bind _formationpositions (CallFunction|GenerateLineFormation (Utilities|Array|Length (Variables|Default|GetFormation)) (Math|Float|Truncate (/ (LocalVariables|GetdistanceStartEnd) _output_get))))
    (for _array_element _formationpositions
      (Utilities|Array|Add _temppositions (+ (Variables|Default|GetnewFormationCenter) _array_element)))
    (for _array_element_2 _temppositions
      (bind _point_ (CallFunction|PointwithRotation (.yaw (Variables|Default|GetformationRotation)) (Variables|Default|GetnewFormationCenter) _array_element_2))
      (Utilities|Array|Add _rotatedpos _point_))
    (for (_array_element_3 _array_index) _formation
      (Utilities|Array|SetArrayElem _formation _array_index (Utilities|Struct|MakeUnitFormationParam (.unitvector _array_element_3) (.unit _array_element_3) (Math|Rotator|MakeRotator 0.0 0.0 (.yaw (Variables|Default|GetformationRotation))) (Utilities|Array|Get(acopy) _rotatedpos _array_index))))
    (return (LocalVariables|GetrotatedPos))))

(fn CalculatePosition
  (params (unitCount :type Integer) (startingPos :type Vector) (endingPos :type Vector) (formationWidth :type Integer))
  (bind _spread (Variables|Default|Getspread))
  (LocalVariables|SetstartPos (Math|Vector|MakeVector (.x startingPos) (.y startingPos) (.z startingPos)))
  (LocalVariables|SetendPos endingPos)
  (for _index (range 0 (- unitCount 1))
    (Utilities|Array|Add (LocalVariables|Getpositions) (Math|Vector|MakeVector (+ (* (/ _index formationWidth) _spread) (.x startingPos)) (+ (* (Math|Integer|%(Integer) _index formationWidth) _spread) (.y startingPos)) (.z startingPos))))
  (return (LocalVariables|Getpositions)))

(fn CalculateSpacing
  (bind _formationpositions (CallFunction|GenerateLineFormation 2 2))
  (return (Math|Vector|Distance(Vector) (Utilities|Array|Get(acopy) _formationpositions) (Utilities|Array|Get(acopy) _formationpositions 1))))

(fn SetTarget
  (params (targetPoint :type Vector))
  (for _array_element 0
    (bind _asunit (Utilities|Casting|CastToUnit (.unit _array_element)))
    (Default|LookatUnit _asunit (Math|Vector|MakeVector (.x targetPoint) (.y targetPoint) (.z targetPoint)))
    (Development|PrintString "Hello")))

(fn ReturnFormationElementbyUnit
  (params (unit :type Character%20Object%20Reference))
  (for _array_element (Variables|Default|GetFormation)
    (if (== (.unit (Utilities|Struct|BreakUnitFormationParam _array_element)) unit)
      (return _array_element))))

(fn SpawnFormationwithActor
  (params (unitCount :type Integer) (Width :type Integer) (formationStartingPoint :type Vector) (owner :type Actor%20Object%20Reference))
  (bind _formation (Variables|Default|Getformation))
  (bind _asplayer (Utilities|Casting|CastToPlayer owner))
  (bind _formationpositions (CallFunction|GenerateLineFormation unitCount Width))
  (for _array_element _formationpositions
    (bind _returnvalue (Game|SpawnActorfromClass "/Game/Blueprints/Unit/UnitPawn.UnitPawn_C" (Math|Transform|MakeTransform (+ formationStartingPoint _array_element) "0, 0, 0" "1,1,1") "Undefined" 0 _asplayer _asplayer))
    (Components|DestroyComponent (Variables|/Script/Engine.Actor|GetRootComponent _returnvalue) (AI|GetAIController _returnvalue))
    (Utilities|Array|Add _formation (Utilities|Struct|MakeUnitFormationParam _array_element 0 "0.000000,0.000000,0.000000" (+ formationStartingPoint _array_element)))
    (Variables|Default|SetformationCenter (+ (+ formationStartingPoint _array_element) (Variables|Default|GetformationCenter))))
  (Variables|Default|SetformationCenter (/ (Variables|Default|GetformationCenter) (Utilities|Array|Length _formation))))

(fn CalculateFirstFormationPosition
  (params (position1 :type Vector) (position2 :type Vector))
  (bind _output_get (LocalVariables|SettransformVector (* (- (Variables|Default|GetnewFormationCenter) (Variables|Default|GetformationCenter)) 0.85)))
  (return (- position1 _output_get) (- position2 _output_get)))

(fn CheckFormationMovement
  (LocalVariables|Setmoving false)
  (for _array_element (Variables|Default|GetFormation)
    (if (>= (+ (.x (Variables|/Script/Engine.MovementComponent|GetVelocity (Pawn|GetMovementComponent (.unit _array_element)))) (.y (Variables|/Script/Engine.MovementComponent|GetVelocity (Pawn|GetMovementComponent (.unit _array_element))))) 3.0)
      (LocalVariables|Setmoving true)
      (else
        (bind _asunit (Utilities|Casting|CastToUnit (.unit _array_element)))
        (Default|LookatUnit _asunit (Variables|Default|GettargetPoint)))))
  (if (LocalVariables|Getmoving)
    (Variables|Default|SetformationMoving true)
    (else
      (Variables|Default|SetformationMoving false))))

(fn SetTargetPoint
  (params (target :type Vector))
  (Variables|Default|SettargetPoint target))