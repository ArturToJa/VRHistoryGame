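; Grippable VR charge that loads the Vive pawn's primary gun when held at its barrel.
; Gripping caches the character and calls its SpawnEqCharge.
; While the gun is in its first state, Tick times ChargeTop's overlap with a component named "Barrel", though only the last overlap result counts.
; On release after LoadingTime, a mesh overlap recheck advances the gun's state and hides the charge mesh.
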(event EventTick
  (params (DeltaSeconds :type Float%20%28single-precision%29))
  (bind _chargetop (Variables|Default|GetChargeTop))
  (bind _character (Variables|Default|GetCharacter))
  (bind _primarygun (Variables|/Game/VRExpansion/Vive/Vive_PawnCharacter.Vive_PawnCharacter_C|GetPrimaryGun _character))
  (Variables|Default|SetIsLoading false)
  (if (Utilities|IsValid _character)
    (if (Utilities|IsValid _primarygun)
      (if (Utilities|Enum|Equal(Enum) (Variables|/Game/VRExpansion/Guns/GunBase.GunBase_C|Getstate _primarygun) "NewEnumerator0")
        (bind _outcomponents (Class|KismetSystemLibrary|ComponentOverlapComponents _chargetop (Transformation|GetWorldTransform _chargetop) (Utilities|Array|MakeArray "ObjectTypeQuery3") "/Script/Engine.StaticMeshComponent" (Utilities|Array|MakeArray self)))
        (for _array_element _outcomponents
          (Variables|Default|SetIsLoading (Utilities|Enum|Equal(Enum) (Utilities|GetObjectName _array_element) "Barrel")))
        (if (Variables|Default|GetIsLoading)
          (Variables|Default|SetTimer (+ (Variables|Default|GetTimer) DeltaSeconds))
          (else
            (Variables|Default|SetTimer 0.0)))))))

(event EventOnGrip
  (params (GrippingController :type Grip%20Motion%20Controller%20Component%20Object%20Reference) (GripInformation :type BP%20Actor%20Grip%20Information%20Structure%20%28by%20ref%29))
  (bind _asvive_pawn_character (Utilities|Casting|CastToVive_PawnCharacter (Components|GetOwner GrippingController)))
  (Variables|Default|SetCharacter _asvive_pawn_character)
  (Default|SpawnEqCharge _asvive_pawn_character))

(event EventOnGripRelease
  (params (ReleasingController :type Grip%20Motion%20Controller%20Component%20Object%20Reference) (GripInformation :type BP%20Actor%20Grip%20Information%20Structure%20%28by%20ref%29) (bWasSocketed :type Boolean))
  (bind _staticmeshcomponent (Variables|Default|GetStaticMeshComponent))
  (if (>= (Variables|Default|GetTimer) (Variables|Default|GetLoadingTime))
    (bind _asvive_pawn_character (Utilities|Casting|CastToVive_PawnCharacter (Components|GetOwner ReleasingController)))
    (if (Utilities|IsValid (Variables|/Game/VRExpansion/Vive/Vive_PawnCharacter.Vive_PawnCharacter_C|GetPrimaryGun _asvive_pawn_character))
      (if (Utilities|Enum|Equal(Enum) (Variables|/Game/VRExpansion/Guns/GunBase.GunBase_C|Getstate (Variables|/Game/VRExpansion/Vive/Vive_PawnCharacter.Vive_PawnCharacter_C|GetPrimaryGun _asvive_pawn_character)) "NewEnumerator0")
        (bind _outcomponents (Class|KismetSystemLibrary|ComponentOverlapComponents _staticmeshcomponent (Transformation|GetWorldTransform _staticmeshcomponent) (Utilities|Array|MakeArray "ObjectTypeQuery3") "/Script/Engine.StaticMeshComponent" (Utilities|Array|MakeArray self)))
        (for _array_element _outcomponents
          (if (Utilities|Enum|Equal(Enum) (Utilities|GetObjectName _array_element) "Barrel")
            (Variables|/Game/VRExpansion/Guns/GunBase.GunBase_C|Setstate (Variables|/Game/VRExpansion/Vive/Vive_PawnCharacter.Vive_PawnCharacter_C|GetPrimaryGun _asvive_pawn_character) "NewEnumerator1")
            (Rendering|SetVisibility (Variables|Default|GetStaticMeshComponent) false false)))))))

(fn ConstructionScript)