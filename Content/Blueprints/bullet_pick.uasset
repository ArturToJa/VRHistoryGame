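; Grippable VR bullet that the player loads by hand into the pawn's primary gun.
; Gripping it calls SpawnEqBullet on the owning Vive_PawnCharacter.
; On release, if the gun is in a specific state, a component overlap query looks for a static mesh named "Barrel".
; A match advances the gun's state and hides the bullet mesh without destroying the actor.
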(event EventOnGrip
  (params (GrippingController :type Grip%20Motion%20Controller%20Component%20Object%20Reference) (GripInformation :type BP%20Actor%20Grip%20Information%20Structure%20%28by%20ref%29))
  (bind _asvive_pawn_character (Utilities|Casting|CastToVive_PawnCharacter (Components|GetOwner GrippingController)))
  (Default|SpawnEqBullet _asvive_pawn_character))

(event EventOnGripRelease
  (params (ReleasingController :type Grip%20Motion%20Controller%20Component%20Object%20Reference) (GripInformation :type BP%20Actor%20Grip%20Information%20Structure%20%28by%20ref%29) (bWasSocketed :type Boolean))
  (bind _staticmeshcomponent (Variables|Default|GetStaticMeshComponent))
  (bind _asvive_pawn_character (Utilities|Casting|CastToVive_PawnCharacter (Components|GetOwner ReleasingController)))
  (if (Utilities|IsValid (Variables|/Game/VRExpansion/Vive/Vive_PawnCharacter.Vive_PawnCharacter_C|GetPrimaryGun _asvive_pawn_character))
    (if (Utilities|Enum|Equal(Enum) (Variables|/Game/VRExpansion/Guns/GunBase.GunBase_C|Getstate (Variables|/Game/VRExpansion/Vive/Vive_PawnCharacter.Vive_PawnCharacter_C|GetPrimaryGun _asvive_pawn_character)) "NewEnumerator1")
      (bind _outcomponents (Class|KismetSystemLibrary|ComponentOverlapComponents _staticmeshcomponent (Transformation|GetWorldTransform _staticmeshcomponent) (Utilities|Array|MakeArray "ObjectTypeQuery3") "/Script/Engine.StaticMeshComponent" (Utilities|Array|MakeArray self)))
      (for _array_element _outcomponents
        (if (Utilities|Enum|Equal(Enum) (Utilities|GetObjectName _array_element) "Barrel")
          (Variables|/Game/VRExpansion/Guns/GunBase.GunBase_C|Setstate (Variables|/Game/VRExpansion/Vive/Vive_PawnCharacter.Vive_PawnCharacter_C|GetPrimaryGun _asvive_pawn_character) "NewEnumerator2")
          (Rendering|SetVisibility (Variables|Default|GetStaticMeshComponent) false false))))))

(fn ConstructionScript)