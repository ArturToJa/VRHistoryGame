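; CommanderMenuActor is a VR command menu that lets the player choose the active formation.
; Each of its two VR buttons, on a state change, passes its own entry from the Formation array to SetActiveFormation on the ViveCharacter.
; The handlers do not check the new button state, and each prints the chosen formation's name as debug output.
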(event OnButtonStateChanged(VRButton)
  (params (ButtonState :type Boolean) (InteractingActor :type Actor%20Object%20Reference) (InteractingComponent :type Primitive%20Component%20Object%20Reference))
  (bind _formation (Variables|Default|GetFormation))
  (bind _output (Utilities|Array|Get(acopy) _formation))
  (Default|SetActiveFormation (Variables|Default|GetViveCharacter) _output)
  (Development|PrintString (Utilities|GetDisplayName _output)))

(event OnButtonStateChanged(VRButton1)
  (params (ButtonState :type Boolean) (InteractingActor :type Actor%20Object%20Reference) (InteractingComponent :type Primitive%20Component%20Object%20Reference))
  (bind _formation (Variables|Default|GetFormation))
  (bind _output (Utilities|Array|Get(acopy) _formation 1))
  (Default|SetActiveFormation (Variables|Default|GetViveCharacter) _output)
  (Development|PrintString (Utilities|GetDisplayName _output)))

(event EventBeginPlay)

(event Collision|EventActorBeginOverlap
  (params (OtherActor :type Actor%20Object%20Reference)))

(event EventTick
  (params (DeltaSeconds :type Float%20%28single-precision%29)))

(fn ConstructionScript)