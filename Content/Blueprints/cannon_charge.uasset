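; Grippable cannon charge that the player loads into a cannon by letting go of it over the barrel.
; On grip release, it queries its mesh's overlaps for Pawn-type static mesh components and picks out any named "CannonBarrel".
; If that component's owning Cannon is in the required GunState, the charge hides its mesh, without being destroyed, and advances the cannon to the next state.
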(event EventOnGrip
  (params (GrippingController :type Grip%20Motion%20Controller%20Component%20Object%20Reference) (GripInformation :type BP%20Actor%20Grip%20Information%20Structure%20%28by%20ref%29)))

(event EventOnGripRelease
  (params (ReleasingController :type Grip%20Motion%20Controller%20Component%20Object%20Reference) (GripInformation :type BP%20Actor%20Grip%20Information%20Structure%20%28by%20ref%29) (bWasSocketed :type Boolean))
  (bind _staticmeshcomponent (Variables|Default|GetStaticMeshComponent))
  (bind _outcomponents (Class|KismetSystemLibrary|ComponentOverlapComponents _staticmeshcomponent (Transformation|GetWorldTransform _staticmeshcomponent) (Utilities|Array|MakeArray "ObjectTypeQuery3") "/Script/Engine.StaticMeshComponent" (Utilities|Array|MakeArray self)))
  (for _array_element _outcomponents
    (if (Utilities|Enum|Equal(Enum) (Utilities|GetObjectName _array_element) "CannonBarrel")
      (bind _ascannon (Utilities|Casting|CastToCannon (Components|GetOwner _array_element)))
      (if (Utilities|Enum|Equal(Enum) (Variables|/Game/Blueprints/Cannon.Cannon_C|GetgunState _ascannon) "NewEnumerator0")
        (Rendering|SetVisibility (Variables|Default|GetStaticMeshComponent) false false)
        (Variables|/Game/Blueprints/Cannon.Cannon_C|SetgunState _ascannon "NewEnumerator1")))))

(fn ConstructionScript)