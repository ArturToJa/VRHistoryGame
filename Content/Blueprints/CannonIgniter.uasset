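; CannonIgniter is a grippable actor that triggers the counter display on a Cannon when held against its igniter.
; On each TickGrip, it overlap-tests its static mesh against Pawn-type static mesh components, ignoring itself, and prints each hit name.
; A component whose display name is "Igniter" has its owner cast to Cannon, and that cannon's Counter is made visible.
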(event EventBeginPlay)

(event EventTick
  (params (DeltaSeconds :type Float%20%28single-precision%29)))

(event EventTickGrip
  (params (GrippingController :type Grip%20Motion%20Controller%20Component%20Object%20Reference) (GripInformation :type BP%20Actor%20Grip%20Information%20Structure%20%28by%20ref%29) (DeltaTime :type Float%20%28single-precision%29))
  (bind _staticmeshcomponent (Variables|Default|GetStaticMeshComponent))
  (bind _outcomponents (Class|KismetSystemLibrary|ComponentOverlapComponents _staticmeshcomponent (Transformation|GetWorldTransform _staticmeshcomponent) (Utilities|Array|MakeArray "ObjectTypeQuery3") "/Script/Engine.StaticMeshComponent" (Utilities|Array|MakeArray self)))
  (for _array_element _outcomponents
    (Development|PrintString (Utilities|GetDisplayName _array_element))
    (if (Utilities|Enum|Equal(Enum) (Utilities|GetDisplayName _array_element) "Igniter")
      (bind _ascannon (Utilities|Casting|CastToCannon (Components|GetOwner _array_element)))
      (Rendering|SetVisibility (Variables|/Game/Blueprints/Cannon.Cannon_C|GetCounter _ascannon) true false))))

(fn ConstructionScript)