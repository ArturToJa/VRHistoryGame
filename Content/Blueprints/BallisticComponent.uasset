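; BallisticComponent is a ballistics helper that predicts how far a projectile travels and how long it takes to land.
; CalculateFire takes pitch in degrees, launch velocity and starting height, then solves the closed-form, drag-free trajectory equation using GravityConstant.
; It returns horizontal Range and TimeToHit, treating impact as the return to zero height.
; It runs no per-frame logic, as BeginPlay and Tick are disabled stubs.
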(event EventBeginPlay)

(event EventTick
  (params (DeltaSeconds :type Float%20%28single-precision%29)))

(fn CalculateFire
  (params (pitch :type Float%20%28single-precision%29) (startingVelocity :type Float%20%28single-precision%29) (startingHeight :type Float%20%28single-precision%29))
  (bind _returnvalue (Math|Trig|Sin(Degrees) pitch))
  (bind _returnvalue_2 (Math|Float|Power startingVelocity 2.0))
  (bind _returnvalue_3 (Math|Trig|Sin(Degrees) pitch))
  (bind _gravityconstant (LocalVariables|GetgravityConstant))
  (bind _gravityconstant_2 (LocalVariables|GetgravityConstant))
  (bind _returnvalue_4 (Math|Float|Power _returnvalue 2.0))
  (bind _returnvalue_5 (* startingVelocity _returnvalue_3))
  (bind _returnvalue_6 (* _gravityconstant 2.0))
  (bind _returnvalue_7 (* _returnvalue_2 _returnvalue_4))
  (bind _returnvalue_8 (* _returnvalue_6 startingHeight))
  (bind _returnvalue_9 (+ _returnvalue_7 _returnvalue_8))
  (bind _returnvalue_10 (Math|Float|Sqrt _returnvalue_9))
  (bind _returnvalue_11 (+ _returnvalue_5 _returnvalue_10))
  (bind _returnvalue_12 (/ _returnvalue_11 _gravityconstant_2))
  (return (* (* startingVelocity (Math|Trig|Cos(Degrees) pitch)) _returnvalue_12) _returnvalue_12))