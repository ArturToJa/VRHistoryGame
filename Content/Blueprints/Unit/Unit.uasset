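; Rifle-armed unit pawn, tinted to its owning player's color, that runs under player or AI control.
; State flags drive a fire and reload cycle on a child-actor rifle, with post-shot reload routed to itself or the UnitAIController.
; AI movement goes through that controller, while CreateCamera adds a runtime camera and reticle for direct aiming.
; Damage only lowers and prints Health; the death collision and ballistic calculation nodes are disconnected.
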(event Custom|UnitFire
  ;[1 1 1] Firing
  (if (Variables|Default|GetweaponLoaded)
    (bind _asrifle_old (Utilities|Casting|CastToRifleOld (Variables|/Script/Engine.ChildActorComponent|GetChildActor (Variables|Default|GetRifle))))
    (Variables|Default|SetisFiring true)
    (Default|Fire _asrifle_old (Variables|Default|Getyaw) (Variables|Default|Getpitch))))

(event Custom|ReloadEvent
  ;[1 1 1] Reloading
  (if (not (Variables|Default|GetweaponLoaded))
    (Variables|Default|SetisReloading true)))

(event Custom|FinishReload
  ;[1 1 1] Reloading
  (Variables|Default|SetisReloading false)
  (Variables|Default|SetweaponLoaded true))

(event Custom|FinishFiring
  (bind _returnvalue (Pawn|GetController))
  ;[1 1 1] Firing
  (Variables|Default|SetisFiring false)
  (Variables|Default|SetweaponLoaded false)
  (if (Class|Controller|IsPlayerController _returnvalue)
    (CallFunction|ReloadEvent)
    (else
      (bind _asunit_aicontroller (Utilities|Casting|CastToUnitAIController _returnvalue))
      (Default|ReloadEvent _asunit_aicontroller))))

(event EventBeginPlay
  ;[1 1 1] Add rifle + reticle
  (bind _returnvalue (UserInterface|CreateWidget "/Game/UI/Reticle.Reticle_C" (Game|GetPlayerController 0)))
  (Variables|Default|SetWidget _returnvalue))

(event Game|Damage|EventAnyDamage
  (params (Damage :type Float%20%28single-precision%29) (DamageType :type Damage%20Type%20Object%20Reference) (InstigatedBy :type Controller%20Object%20Reference) (DamageCauser :type Actor%20Object%20Reference))
  ;[1 1 1] Receive Damage
  (CallFunction|TakeDamage Damage))

(fn ConstructionScript
  (bind _owningplayer (Variables|Default|GetOwningPlayer))
  (bind _playercolor (Variables|/Game/VRExpansion/Vive/Vive_PawnCharacter.Vive_PawnCharacter_C|GetPlayerColor _owningplayer))
  (Rendering|Material|SetVectorParameterValueonMaterials (Variables|Character|GetMesh self) "BodyColor" (Math|Vector|MakeVector (Math|Conversions|ToFloat(Byte) (.r _playercolor)) (Math|Conversions|ToFloat(Byte) (.g _playercolor)) (Math|Conversions|ToFloat(Byte) (.b _playercolor))))
  (Transformation|AttachComponentToComponent (Variables|Default|GetRifle) (Variables|Character|GetMesh) "weapon" "SnapToTarget" "SnapToTarget" "SnapToTarget" true)
  (Variables|Default|SetweaponLoaded true))

(fn SetYaw
  (params (yaw :type Float%20%28single-precision%29))
  (Variables|Default|Setyaw yaw))

(fn SetPitch
  (params (pitch :type Float%20%28single-precision%29))
  (Variables|Default|Setpitch pitch))

(fn CreateCamera
  (bind _returnvalue (AddComponent|AddCameraComponent false))
  (Variables|/Script/Engine.CameraComponent|SetbUsePawnControlRotation _returnvalue true)
  (Transformation|AddLocalOffset _returnvalue "20.000000, 0,70.000000" false true)
  (bind _asrifle_old (Utilities|Casting|CastToRifleOld (Variables|/Script/Engine.ChildActorComponent|GetChildActor (Variables|Default|GetRifle))))
  (Default|SetCamera _asrifle_old _returnvalue)
  (UserInterface|Viewport|AddtoViewport (Variables|Default|GetWidget) 0))

(fn MoveUnit
  (params (NewPosition :type Vector%202D%20Structure))
  (bind _asunit_aicontroller (Utilities|Casting|CastToUnitAIController (AI|GetAIController self)))
  (Default|Moveto _asunit_aicontroller NewPosition))

(fn LookatUnit
  (params (location :type Vector))
  (Transformation|SetActorRotation (Math|Interpolation|RInterpTo (Math|Rotator|MakeRotator 0.0 0.0 (.yaw (Math|Rotator|FindLookatRotation (Transformation|GetActorLocation) location))) (Transformation|GetActorRotation) (Utilities|Time|GetWorldDeltaSeconds) 3.0)))

(fn GetRifle
  (bind _asrifle_old (Utilities|Casting|CastToRifleOld (Variables|/Script/Engine.ChildActorComponent|GetChildActor (Variables|Default|GetRifle))))
  (return _asrifle_old))

(fn IsAlive
  (return (> (Variables|Default|GetHealth) 0.0)))

(fn TakeDamage
  (params (Damage :type Float%20%28single-precision%29))
  (bind _output_get (Variables|Default|SetHealth (- (Variables|Default|GetHealth) Damage)))
  (Development|PrintString (Utilities|String|ToString(Float) _output_get)))