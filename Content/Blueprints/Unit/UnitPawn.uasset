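; Unit pawn for player-owned units, with a skeletal mesh and weapon state flags.
; The construction script tints the mesh's BodyColor material parameter with the owning player's color and forces a fixed LOD.
; Reset sets the weapon to loaded and clears the reloading, firing and aiming flags.
; GetRifle is an empty stub, and the nodes that attach to the weapon socket are disconnected and never run.
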(fn ConstructionScript
  (bind _owningplayer (Variables|Default|GetOwningPlayer))
  (bind _playercolor (Variables|/Game/Blueprints/RTSCamera/Player.Player_C|GetPlayerColor _owningplayer))
  (Rendering|Material|SetVectorParameterValueonMaterials (Variables|Default|GetSkeletalMesh) "BodyColor" (Math|Vector|MakeVector (Math|Conversions|ToFloat(Byte) (.r _playercolor)) (Math|Conversions|ToFloat(Byte) (.g _playercolor)) (Math|Conversions|ToFloat(Byte) (.b _playercolor))))
  (Components|SkinnedMesh|SetForcedLOD (Variables|Default|GetSkeletalMesh) 7))

(fn GetRifle)