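; Behavior tree task that finds a nearby Unit and stores it as the TargetUnit blackboard value.
; On tick, it sphere-overlaps Pawns of class Unit around the owning Unit, excluding itself, with a radius slightly beyond its rifle's range.
; It takes the first overlap result without sorting by distance or filtering by team, then finishes with the overlap's success flag.
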(event EventTick
  (params (OwnerActor :type Actor%20Object%20Reference) (DeltaSeconds :type Float%20%28single-precision%29))
  (bind _asunit (Utilities|Casting|CastToUnit OwnerActor))
  (bind _rifle (Default|GetRifle _asunit))
  (bind (_outactors _returnvalue) (Collision|SphereOverlapActors (Transformation|GetActorLocation _asunit) (+ (Variables|/Game/Blueprints/RifleOld.RifleOld_C|GetRange _rifle) 2e+02) (Utilities|Array|MakeArray "ObjectTypeQuery3") "/Game/Blueprints/Unit/Unit.Unit_C" (Utilities|Array|MakeArray _asunit)))
  (Class|BTFunctionLibrary|SetBlackboardValueasObject (Variables|Default|GetTargetUnit) (Utilities|Array|Get(acopy) _outactors))
  (AI|BehaviorTree|FinishExecute _returnvalue))