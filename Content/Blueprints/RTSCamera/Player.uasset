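; RTS player pawn providing the camera and unit commands, with screen-edge panning while in control.
; Left mouse drives box selection through PlayerHud and passes the cursor hit to the Formation as its target.
; Right-drag deprojects the cursor to preview formation slots and facing with debug shapes, then moves the Formation on release.
; Space possesses the first selected unit, and SetControlToThis restores camera control.
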(event EventBeginPlay
  (bind _returnvalue (Game|GetPlayerController 0))
  ;[1 1 1] Initialization
  (Utilities|FlowControl|Sequence
    (:then_0
      (Input|EnableInput _returnvalue)
      (Variables|/Script/Engine.PlayerController|SetbShowMouseCursor _returnvalue true)
      (bind _asplayer_hud (Utilities|Casting|CastToPlayerHud (HUD|GetHUD _returnvalue)))
      (Default|SetPlayerPawn _asplayer_hud self)
      (Default|SetSpringArm (Variables|Default|GetSmoothZoom) (Variables|Default|GetSpringArm)))))

(event EventTick
  (params (DeltaSeconds :type Float%20%28single-precision%29))
  (bind _returnvalue (Game|GetPlayerController 0))
  (bind _position1 (Variables|Default|Getposition1))
  (bind (_worldlocation _worlddirection) (Game|Player|ConvertMouseLocationToWorldSpace _returnvalue))
  (bind _z (Math|Vector|BreakVector _worlddirection))
  (bind _z_2 (Math|Vector|BreakVector _worldlocation))
  (bind _returnvalue_2 (/ _z_2 _z))
  (bind _returnvalue_3 (* _worlddirection _returnvalue_2))
  (bind _returnvalue_4 (* _returnvalue_3 -1.0))
  (bind _returnvalue_5 (+ _worldlocation _returnvalue_4))
  (bind _returnvalue_6 (Math|Vector|MakeVector (.x _returnvalue_5) (.y _returnvalue_5) (.z _position1)))
  ;[1 1 1] Move camera border
  (Utilities|FlowControl|Sequence
    (:then_0
      (if (Variables|Default|GetInControl)
        (bind _returnvalue_7 (Class|WidgetLayoutLibrary|GetMousePositiononViewport))
        (bind _deltas (CallFunction|GetDeltas _returnvalue_7))
        (Transformation|AddActorLocalOffset (Math|Vector|MakeVector (.x _deltas) (.y _deltas) 0.0) false false)))
    (:then_1
      (bind _returnvalue_8 (Class|WidgetLayoutLibrary|GetMousePositiononPlatform))
      (if (Variables|Default|GetRightButtonPressed)
        (Rendering|Debug|DrawDebugCircle (Variables|Default|Getposition1) 43.5 24 "(R=0.127743,G=1.000000,B=0.000000,A=1.000000)" 0.05 8.0 "1.000000,0.000000,0.000000" "0.000000,1.000000,0.000000")
        (if (not (Math|Vector|Equal(Vector) _returnvalue_8 (Variables|Default|Getposition1mouse) 0.0001))
          (bind _output_get (Variables|Default|Setposition2 _returnvalue_6))
          (Rendering|Debug|DrawDebugCircle _output_get 43.5 24 "(R=0.079982,G=1.000000,B=0.000000,A=1.000000)" 0.05 8.0 "1.000000,0.000000,0.000000" "0.000000,1.000000,0.000000")
          (bind _output_get_2 (Variables|Default|SetposMiddle (/ (+ _returnvalue_6 (Variables|Default|Getposition1)) 2.0)))
          (Rendering|Debug|DrawDebugCircle _output_get_2 43.5 24 "(R=1.000000,G=0.988924,B=0.000000,A=1.000000)" 0.05 8.0 "1.000000,0.000000,0.000000" "0.000000,1.000000,0.000000")
          (bind (_x_ _y_) (CallFunction|RotationArrow (.X (Math|Vector|BreakVector _output_get_2)) (.Y (Math|Vector|BreakVector _output_get_2)) 3e+02 (- (.yaw (Math|Rotator|FindLookatRotation (Variables|Default|Getposition1) (Variables|Default|Getposition2))) 9e+01)))
          (bind (_x__2 _y__2) (CallFunction|RotationArrow (.X (Math|Vector|BreakVector _output_get_2)) (.Y (Math|Vector|BreakVector _output_get_2)) 5e+03 (- (.yaw (Math|Rotator|FindLookatRotation (Variables|Default|Getposition1) (Variables|Default|Getposition2))) 9e+01)))
          (Variables|Default|SettargetPoint (Math|Vector|MakeVector _x__2 _y__2 (.Z (Math|Vector|BreakVector _output_get_2))))
          (Rendering|Debug|DrawDebugArrow _output_get_2 (Math|Vector|MakeVector _x_ _y_ (.Z (Math|Vector|BreakVector _output_get_2))) 6.0 "(R=1.000000,G=0.974420,B=0.000000,A=1.000000)" 0.05 6.0)
          (bind _positions (Default|DynamicPositionFormation (Variables|Default|Getformation) (Variables|Default|Getposition1) (Variables|Default|Getposition2)))
          (for _array_element _positions
            (Rendering|Debug|DrawDebugCircle _array_element 43.5 24 "(R=0.963065,G=0.000000,B=1.000000,A=1.000000)" 0.05 8.0 "1.000000,0.000000,0.000000" "0.000000,1.000000,0.000000")))))))

(event Input|MouseEvents|LeftMouseButton
  (params (Key :type Key%20Structure :default "None"))
  ;[1 1 1] Select units
  (:Pressed
    (if (Variables|Default|GetInControl) :!label _label
      (bind _asplayer_hud (Utilities|Casting|CastToPlayerHud (HUD|GetHUD (Game|GetPlayerController 0))))
      (Default|SelectionMode _asplayer_hud)
      (for _array_element (Variables|/Game/Blueprints/RTSCamera/PlayerHud.PlayerHud_C|GetSelectedActors _asplayer_hud)
        (bind _newparam (Default|ReturnFormationElementbyUnit (Variables|Default|Getformation) _array_element)))))
  (:Released
    (goto _label)))

(event Input|KeyboardEvents|SpaceBar
  (params (Key :type Key%20Structure :default "None"))
  ;[1 1 1] Set control to selected unit
  (:Pressed
    (bind _asplayer_hud (Utilities|Casting|CastToPlayerHud (HUD|GetHUD (Game|GetPlayerController 0))))
    (CallFunction|SetControltoUnit (Utilities|Array|Get(acopy) (Variables|/Game/Blueprints/RTSCamera/PlayerHud.PlayerHud_C|GetSelectedActors _asplayer_hud)))))

(event Input|MouseEvents|RightMouseButton
  (params (Key :type Key%20Structure :default "None"))
  ;[1 1 1] Unit control - Fire and move
  (:Pressed
    (Variables|Default|SetRightButtonPressed true)))

(event Input|KeyboardEvents|C
  (params (Key :type Key%20Structure :default "None"))
  (:Pressed
    (Class|KismetSystemLibrary|FlushDebugStrings :!label _label))
  (:Released
    (goto _label)))

(event Input|MouseEvents|MouseWheelDown
  (params (Key :type Key%20Structure :default "None"))
  ;[1 1 1] Scroll logic
  (:Pressed
    (if (Variables|Default|GetRightButtonPressed)
      (Variables|Default|SetformationRotation (Math|Rotator|MakeRotator 0.0 0.0 (- (.yaw (Variables|Default|GetformationRotation)) 7.5))))))

(event Input|MouseEvents|MouseWheelUp
  (params (Key :type Key%20Structure :default "None"))
  ;[1 1 1] Scroll logic
  (:Pressed
    (if (Variables|Default|GetRightButtonPressed)
      (Variables|Default|SetformationRotation (Math|Rotator|MakeRotator 0.0 0.0 (+ (.yaw (Variables|Default|GetformationRotation)) 7.5))))))

(event Input|MouseEvents|LeftMouseButton
  (params (Key :type Key%20Structure :default "None"))
  ;[1 1 1] Move camera border
  (:Released
    (Default|SetTarget (Variables|Default|Getformation) (.location (.HitResult (Game|Player|GetHitResultUnderCursorbyChannel (Game|GetPlayerController 0) "TraceTypeQuery1" true))))))

(event Input|MouseEvents|RightMouseButton
  (params (Key :type Key%20Structure :default "None"))
  (:Pressed
    (Variables|Default|SetRightButtonPressed true)
    (Variables|Default|Setposition1 (.impactpoint (.HitResult (Game|Player|GetHitResultUnderCursorbyChannel (Game|GetPlayerController 0) "TraceTypeQuery1" true))))
    (bind _returnvalue (Class|WidgetLayoutLibrary|GetMousePositiononPlatform))
    (Variables|Default|Setposition1mouse _returnvalue)
    (bind _returnvalue_2 (Class|WidgetLayoutLibrary|GetMousePositiononPlatform))
    (if (Variables|Default|GetRightButtonPressed)
      (Rendering|Debug|DrawDebugCircle (Variables|Default|Getposition1) 43.5 24 "(R=0.127743,G=1.000000,B=0.000000,A=1.000000)" 0.05 8.0 "1.000000,0.000000,0.000000" "0.000000,1.000000,0.000000")))
  (:Released
    (Variables|Default|SetRightButtonPressed false)
    (Default|MoveFormation (Variables|Default|Getformation) (Variables|Default|Getposition1) (Variables|Default|Getposition2) (Variables|Default|GettargetPoint))))

(fn ConstructionScript)

(fn GetViewportScaled
  (bind _returnvalue (Viewport|GetViewportSize))
  (bind _returnvalue_2 (Class|WidgetLayoutLibrary|GetViewportScale))
  (return (Math|Vector2D|MakeVector2D (/ (.x _returnvalue) _returnvalue_2) (/ (.y _returnvalue) _returnvalue_2))))

(fn GetDeltas
  (params (MousePosition :type Vector%202D%20Structure))
  (LocalVariables|SetDeltaX 0.0)
  (LocalVariables|SetDeltaY 0.0)
  (bind _viewport_scaled (CallFunction|GetViewportScaled))
  (Utilities|FlowControl|Sequence
    (:then_0
      ;[1 1 1] Left-Right camera movement
      (if (< (.x MousePosition) (Variables|Default|GetBorderSize-Const))
        (LocalVariables|SetDeltaX (+ (* (Variables|Default|GetCameraMoveSpeed) -1.0) (LocalVariables|GetDeltaX)))))
    (:then_1
      (if (> (.x MousePosition) (- (.x _viewport_scaled) (Variables|Default|GetBorderSize-Const)))
        (LocalVariables|SetDeltaX (+ (Variables|Default|GetCameraMoveSpeed) (LocalVariables|GetDeltaX)))))
    (:then_2
      ;[1 1 1] Up-Down camera movement
      (if (< (.y MousePosition) (Variables|Default|GetBorderSize-Const))
        (LocalVariables|SetDeltaY (+ (Variables|Default|GetCameraMoveSpeed) (LocalVariables|GetDeltaY)))))
    (:then_3
      (if (> (.y MousePosition) (- (.y _viewport_scaled) (Variables|Default|GetBorderSize-Const)))
        (LocalVariables|SetDeltaY (+ (* (Variables|Default|GetCameraMoveSpeed) -1.0) (LocalVariables|GetDeltaY)))))
    (:then_4
      (return (Math|Vector2D|MakeVector2D (LocalVariables|GetDeltaY) (LocalVariables|GetDeltaX))))))

(fn SetControltoThis
  (params (AIUnit :type Unit%20Object%20Reference))
  (bind _returnvalue (Game|GetPlayerController 0))
  (Pawn|Possess _returnvalue self)
  (Variables|/Script/Engine.PlayerController|SetbShowMouseCursor _returnvalue true)
  (Variables|Default|SetInControl true))

(fn SetControltoUnit
  (params (UnitReference :type Unit%20Object%20Reference))
  (bind _returnvalue (Game|GetPlayerController 0))
  (Pawn|Possess _returnvalue UnitReference)
  (Variables|/Script/Engine.PlayerController|SetbShowMouseCursor _returnvalue false)
  (Variables|Default|SetInControl false))

(fn GetArrowsCameraOffset
  (bind _returnvalue (Game|GetPlayerController 0))
  (bind _cameramovespeed (Variables|Default|GetCameraMoveSpeed))
  (bind _returnvalue_2 (Game|Player|IsInputKeyDown _returnvalue "Right"))
  (bind _returnvalue_3 (Game|Player|IsInputKeyDown _returnvalue "Up"))
  (bind _returnvalue_4 (Game|Player|IsInputKeyDown _returnvalue "Down"))
  (bind _returnvalue_5 (Game|Player|IsInputKeyDown _returnvalue "Left"))
  (bind _returnvalue_6 (* _cameramovespeed -1.0))
  (return (+ (* (Math|Conversions|ToFloat(Boolean) _returnvalue_4) _returnvalue_6) (* (Math|Conversions|ToFloat(Boolean) _returnvalue_3) _cameramovespeed)) (+ (* _returnvalue_6 (Math|Conversions|ToFloat(Boolean) _returnvalue_5)) (* _cameramovespeed (Math|Conversions|ToFloat(Boolean) _returnvalue_2))) (Math|Boolean|ORBoolean _returnvalue_4 _returnvalue_3 _returnvalue_5 _returnvalue_2)))

(fn CalculatePosition
  (params (self2 :type Character%20Object%20Reference) (index :type Integer) (X :type Float%20%28single-precision%29) (Y :type Float%20%28single-precision%29))
  (bind _capsulecomponent (Variables|/Script/Engine.Character|GetCapsuleComponent self2))
  (bind _returnvalue (Components|Capsule|GetScaledCapsuleRadius _capsulecomponent))
  (bind _returnvalue_2 (* _returnvalue 3.0))
  (return (+ (* (/ index 2) _returnvalue_2) X) (+ (* (Math|Integer|%(Integer) index 2) _returnvalue_2) Y)))

(fn CalculatePositionWidth
  (params (unitWidth :type Float%20%28single-precision%29) (index :type Integer) (X :type Float%20%28single-precision%29) (Y :type Float%20%28single-precision%29) (formationWidth :type Integer))
  (bind _returnvalue (* unitWidth 2.5))
  (return (+ (* (Math|Integer|%(Integer) index formationWidth) _returnvalue) Y) (+ (* (/ index formationWidth) _returnvalue) X)))

(fn RotationArrow
  (params (X :type Float%20%28single-precision%29) (Y :type Float%20%28single-precision%29) (range :type Float%20%28single-precision%29) (angle :type Float%20%28single-precision%29))
  (return (+ X (* range (Math|Trig|Cos(Degrees) angle))) (+ Y (* range (Math|Trig|Sin(Degrees) angle)))))

(fn RotateAround
  (params (center :type Vector) (rotation :type Rotator) (distance :type Float%20%28single-precision%29))
  (return (+ (Math|Vector|GetForwardVector rotation) (* center distance))))

(fn PointwithRotation
  (params (angle :type Float%20%28single-precision%29) (centerPoint :type Vector) (orgPoint :type Vector))
  (bind _returnvalue (Math|Trig|Cos(Degrees) angle))
  (bind _returnvalue_2 (Math|Trig|Sin(Degrees) angle))
  (bind _returnvalue_3 (- (.y orgPoint) (.y centerPoint)))
  (bind _returnvalue_4 (- (.x orgPoint) (.x centerPoint)))
  (return (Math|Vector|MakeVector (+ (- (* _returnvalue _returnvalue_4) (* _returnvalue_2 _returnvalue_3)) (.x centerPoint)) (+ (* _returnvalue_4 _returnvalue_2) (* _returnvalue_3 _returnvalue) (.y centerPoint)) (.z orgPoint))))