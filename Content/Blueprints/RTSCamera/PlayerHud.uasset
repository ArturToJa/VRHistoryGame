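; RTS HUD that handles box and single selection of the player's units.
; SelectionMode records the mouse anchor and toggles a gate, through which DrawHUD draws a translucent green rectangle to the cursor and reselects the units inside it each frame.
; SetSelectedActors, shared with SelectSingleUnit, keeps only units owned by the stored player pawn and toggles their selection circles as the selection changes.
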(event Custom|SelectionMode
  (bind _returnvalue (Game|GetPlayerController 0))
  (bind (_locationx _locationy) (Game|Player|GetMousePosition _returnvalue))
  (Variables|Default|SetAnchorPoint (Math|Vector2D|MakeVector2D _locationx _locationy))
  (Utilities|FlowControl|Gate true) ; enters at Toggle
)

(event EventDrawHUD
  (params (SizeX :type Integer) (SizeY :type Integer))
  (bind _returnvalue (Game|GetPlayerController 0))
  (bind _anchorpoint (Variables|Default|GetAnchorPoint))
  (bind (_x _y) (Math|Vector2D|BreakVector2D _anchorpoint))
  (bind (_locationx _locationy) (Game|Player|GetMousePosition _returnvalue))
  (bind _returnvalue_2 (- (Math|Vector2D|MakeVector2D _locationx _locationy) _anchorpoint))
  (Utilities|FlowControl|Gate true
    (:Exit
      (CallFunction|SetSelectedActors (Class|HUD|GetActorsinSelectionRectangle "/Game/Blueprints/Unit/Unit.Unit_C" (Variables|Default|GetAnchorPoint) (Math|Vector2D|MakeVector2D _locationx _locationy) false false))
      (HUD|DrawRect "(R=0.261000,G=1.000000,B=0.235000,A=0.400000)" _x _y (.x _returnvalue_2) (.y _returnvalue_2)))))

(fn ConstructionScript)

(fn SetPlayerPawn
  (params (PlayerReference :type Player%20Object%20Reference))
  (Variables|Default|SetPlayerPawn PlayerReference))

(fn SetCurrentSelection
  (params (Visible :type Boolean))
  (for _array_element (Variables|Default|GetSelectedActors)
    (bind _asunit (Utilities|Casting|CastToUnit _array_element))
    (Rendering|SetVisibility (Variables|/Game/Blueprints/Unit/Unit.Unit_C|GetSelectionCircle _asunit) Visible false)))

(fn SelectSingleUnit
  (params (UnitToSelect :type Unit%20Object%20Reference))
  (CallFunction|SetSelectedActors (Utilities|Array|MakeArray UnitToSelect)))

(fn SetSelectedActors
  (params (SelectedUnits :type Array%20of%20Actor%20Object%20References))
  (CallFunction|SetCurrentSelection false)
  (Utilities|Array|Clear (Variables|Default|GetSelectedActors))
  (for _array_element SelectedUnits
    (bind _asunit (Utilities|Casting|CastToUnit _array_element))
    (if (== (Variables|/Game/Blueprints/Unit/Unit.Unit_C|GetOwningPlayer _asunit) (Variables|Default|GetPlayerPawn))
      (Utilities|Array|Add (Variables|Default|GetSelectedActors) _asunit)))
  (CallFunction|SetCurrentSelection true))