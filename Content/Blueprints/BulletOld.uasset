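; BulletOld is a projectile actor that damages Units on overlap.
; At BeginPlay, its BallisticComponent computes time-to-hit from pitch, initial speed scaled down by 100 and spawn height, which becomes the lifespan if the player pawn is a Unit.
; Overlapping a Unit applies fixed damage credited to player controller 0, destroys the bullet and prints the Unit's name.
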(event EventBeginPlay
  (bind _timetohit (Default|CalculateFire (Variables|Default|GetBallisticComponent) (.pitch (Transformation|GetActorRotation)) (/ (Variables|/Script/Engine.ProjectileMovementComponent|GetInitialSpeed (Variables|Default|GetProjectileMovement)) 1e+02) (.z (Transformation|GetActorLocation))))
  (Utilities|Casting|CastToUnit (Game|Player|GetPlayerPawn 0))
  (Actor|SetLifeSpan _timetohit))

(event Collision|EventActorBeginOverlap
  (params (OtherActor :type Actor%20Object%20Reference))
  (bind _asunit (Utilities|Casting|CastToUnit OtherActor))
  (Game|Damage|ApplyDamage _asunit 34.0 (Game|GetPlayerController 0) self)
  (Actor|DestroyActor)
  (Development|PrintString (Utilities|GetDisplayName _asunit)))

(event EventTick
  (params (DeltaSeconds :type Float%20%28single-precision%29)))

(fn ConstructionScript)