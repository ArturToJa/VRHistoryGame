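; RifleOld is a rifle Blueprint that fires projectile bullets from its muzzle socket.
; Fire spawns a BulletOld using the passed pitch and a yaw offset from the rifle's rotation, corrected by 90 degrees.
; ShowMuzzle reveals the muzzle flash through a DoOnce, but its hide-and-reset logic is disconnected.
; Construction forces the rifle mesh LOD, and SetCamera stores a camera used only by leftover, unexecuted hitscan trace code.
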(event Custom|Fire
  (params (Yaw :type Float%20%28single-precision%29) (Pitch :type Float%20%28single-precision%29))
  (bind _rifle (Variables|Default|GetRifle))
  (bind _returnvalue (Transformation|GetWorldRotation _rifle))
  (Game|SpawnActorfromClass "/Game/Blueprints/BulletOld.BulletOld_C" (Math|Transform|MakeTransform (Transformation|GetSocketLocation _rifle "Muzzleflash") (Math|Rotator|MakeRotator (.roll _returnvalue) Pitch (- (+ Yaw (.yaw _returnvalue)) 9e+01)) "1,1,1") "Undefined" 0 0))

(fn ConstructionScript
  (Components|SkinnedMesh|SetForcedLOD (Variables|Default|GetRifle) 7))

(fn ShowMuzzle
  (Utilities|FlowControl|DoOnce false
    (:Completed
      (Rendering|SetVisibility (Variables|Default|GetMuzzleflash) true false))))

(fn SetCamera
  (params (Cam :type Camera%20Component%20Object%20Reference))
  (Variables|Default|SetCamera Cam))