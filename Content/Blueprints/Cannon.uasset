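; A VR cannon actor that fires projectiles at an elevation set by a lever, controlled with physical buttons.
; Every tick, a text display shows the lever angle divided by three, which also becomes the projectile's pitch; roll and yaw follow the barrel.
; The fire button spawns a projectile with sound only in one GunState, then resets that state.
; A cheat button sets the firing state directly.
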(event OnButtonStateChanged(VRButton)
  (params (ButtonState :type Boolean) (InteractingActor :type Actor%20Object%20Reference) (InteractingComponent :type Primitive%20Component%20Object%20Reference))
  (bind _cannonbarrel (Variables|Default|GetCannonBarrel))
  (bind _returnvalue (Transformation|GetWorldTransform _cannonbarrel))
  (bind (_location _rotation) (Math|Transform|BreakTransform _returnvalue))
  (if (Utilities|Enum|Equal(Enum) (Variables|Default|GetgunState) "NewEnumerator2")
    (Game|SpawnActorfromClass "/Game/VRExpansion/FirstPersonBP/FirstPersonBP/Blueprints/FirstPersonProjectile.FirstPersonProjectile_C" (Math|Transform|MakeTransform _location (Math|Rotator|MakeRotator (.roll _rotation) (/ (Variables|/Script/VRExpansionPlugin.VRLeverComponent|GetCurrentLeverAngle (Variables|Default|GetVRLever1)) 3.0) (.yaw _rotation)) "1.000000,1.000000,1.000000") "AdjustIfPossibleButAlwaysSpawn" 0 0)
    (Audio|PlaySoundatLocation "/Game/Assets/Cannon/Cannon+5.Cannon+5" (Transformation|GetWorldLocation _cannonbarrel) "0, 0, 0" 1.0 1.0 0.0 0 0 0) ; Play firing sound
    (Variables|Default|SetgunState "NewEnumerator0")))

(event OnButtonStateChanged(cheatbutton)
  (params (ButtonState :type Boolean) (InteractingActor :type Actor%20Object%20Reference) (InteractingComponent :type Primitive%20Component%20Object%20Reference))
  (Variables|Default|SetgunState "NewEnumerator2"))

(event EventBeginPlay)

(event Collision|EventActorBeginOverlap
  (params (OtherActor :type Actor%20Object%20Reference)))

(event EventTick
  (params (DeltaSeconds :type Float%20%28single-precision%29))
  (Rendering|Components|TextRender|SetText (Variables|Default|GetTextRender) (Utilities|Text|ToText(Float) (/ (Variables|/Script/VRExpansionPlugin.VRLeverComponent|GetCurrentLeverAngle (Variables|Default|GetVRLever1)) 3.0) "ToZero" false true 2 324 1 1)))

(fn ConstructionScript)